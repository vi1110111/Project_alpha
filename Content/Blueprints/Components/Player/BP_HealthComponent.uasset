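; Health component for Bot actors that applies incoming damage and handles death.
; On begin play it binds to the owning Bot's damage event, then uses math expressions to reduce Health by armor-mitigated damage and wear down Armor.
; At zero health it sets Dead, whose RepNotify disables capsule collision, ragdolls the mesh and destroys the Bot after a short timer.
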(event Custom|OnBotTakeAndeDamage
  (params (DamagedActor :type Actor%20Object%20Reference) (Damage :type Float%20%28single-precision%29) (DamageType :type Damage%20Type%20Object%20Reference) (InstigatedBy :type Controller%20Object%20Reference) (DamageCauser :type Actor%20Object%20Reference))
  (CallFunction|ApplyDamage Damage))

(event EventBeginPlay
  (bind _asbot (Utilities|Casting|CastToBot (Components|GetOwner)))
  (bind _output_get (Variables|Default|SetBot _asbot))
  (EventDispatchers|AssignOnTakeAnyDamage _output_get (EventDispatchers|CreateEvent :!event Custom|OnBotTakeAndeDamage)))

(event EventTick
  (params (DeltaSeconds :type Float%20%28single-precision%29)))

(fn ApplyDamage
  (params (Damage :type Float%20%28double-precision%29))
  (bind _output_get (LocalVariables|SetLocal_damage Damage))
  (Development|PrintString (Utilities|String|Append "Damage: " (Utilities|String|ToString(Float) _output_get)) true true "(R=1.000000,G=0.000000,B=0.089263,A=1.000000)")
  (Variables|Default|SetHealth (|({B489C785-4F01-6A40-8345-8797B14C0AD0}-({D397D8F7-4160-C3C8-8E39-4A852BEB457A}*(1-({D3B1E775-4832-81A6-8365-138A1C4A8E49}/200))))))
  (Variables|Default|SetArmor (|(max(({D3B1E775-4832-81A6-8365-138A1C4A8E49}-({D397D8F7-4160-C3C8-8E39-4A852BEB457A}*2)),0))))
  (if (<= (Variables|Default|GetHealth) 0.0)
    (Variables|Default|SetDead true)))

(fn OnRepDead
  (bind _bot (Variables|Default|GetBot))
  (bind _mesh (Variables|/Script/Engine.Character|GetMesh _bot))
  (Development|PrintString "Minus Rusnya" true true "(R=0.444301,G=0.000000,B=1.000000,A=1.000000)" 1e+01)
  (Collision|SetCollisionEnabled (Variables|/Script/Engine.Character|GetCapsuleComponent _bot) "NoCollision")
  (Physics|SetSimulatePhysics _mesh true)
  (Collision|SetCollisionEnabled _mesh "QueryAndPhysics")
  (Collision|SetCollisionResponsetoAllChannels _mesh "ECR_Block")
  (Utilities|Time|SetTimerbyFunctionName 0 "Sweep" 3.0))

(fn Sweep
  (Actor|DestroyActor (Variables|Default|GetBot)))