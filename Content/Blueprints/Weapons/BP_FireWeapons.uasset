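; Firearm weapon Blueprint that extends a parent weapon's Use Weapon with firing, ammo reporting and reloading.
; A successful use spawns FireProjectile if one is set, otherwise line-traces from the My_Character camera along the owner's forward vector and applies point damage.
; An empty magazine sets Reloading, whose RepNotify disables firing and starts a timer to refill from TotalAmmo, using class-default CurrentAmmo as magazine size.
; Debug prints and trace drawing remain in place.
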(event EventBeginPlay
  (|CallParentFunction) ; This node is disabled and will not be called.\nDrag off pins to build functionality.
)

(event Collision|EventActorBeginOverlap
  (params (OtherActor :type Actor%20Object%20Reference))
  (|CallParentFunction OtherActor) ; This node is disabled and will not be called.\nDrag off pins to build functionality.
)

(event EventTick
  (params (DeltaSeconds :type Float%20%28single-precision%29))
  (|CallParentFunction DeltaSeconds) ; This node is disabled and will not be called.\nDrag off pins to build functionality.
)

(fn ConstructionScript
  (|CallParentFunction))

(fn UseWeapon
  (bind _used (|CallParentFunction))
  (Development|PrintString (Utilities|String|Append (Utilities|String|ToString(Integer) (Variables|Default|GetCurrentAmmo)) "/" (Utilities|String|ToString(Integer) (Variables|Default|GetTotalAmmo))) true true "(R=0.000000,G=0.660000,B=1.000000,A=1.000000)" 1.0)
  (if _used
    (if (Utilities|IsValidClass (Variables|Default|GetFireProjectile))
      (CallFunction|SpawnShootProjectile)
      (else
        (CallFunction|GetFireTrace)))
    (if (== (Variables|Default|GetCurrentAmmo) 0)
      (Variables|Reload|SetReloading true)
      (return true)
      (else
        (return true)))
    (elif (<= (Variables|Default|GetCurrentAmmo) 0)
      (Variables|Reload|SetReloading true)
      (return false)
      (else
        (return false)))))

(fn GetFireTrace
  (bind _asmy_character (Utilities|Casting|CastToMy_Character (Game|GetInstigator))
    (:then
      (bind _outhit (Collision|LineTraceForObjects (Transformation|GetWorldLocation (Variables|/Game/Blueprints/Character/My_Character.My_Character_C|GetFirstPersonCamera _asmy_character)) (+ (Transformation|GetWorldLocation (Variables|/Game/Blueprints/Character/My_Character.My_Character_C|GetFirstPersonCamera _asmy_character)) (* (Transformation|GetActorForwardVector (Components|GetOwner)) (Math|Conversions|ToVector(Float) 1e+05))) (Utilities|Array|MakeArray "ObjectTypeQuery1" "ObjectTypeQuery2" "ObjectTypeQuery3") false (Utilities|Array|MakeArray self (Game|GetInstigator)) "ForDuration"))
      (Game|Damage|ApplyPointDamage (.HitActor (Collision|BreakHitResult _outhit)) (Variables|Default|GetDamage) (Math|Vector|GetUnitDirection(Vector) (.TraceEnd (Collision|BreakHitResult _outhit)) (.TraceStart (Collision|BreakHitResult _outhit))) _outhit (Game|GetInstigatorController) self)
      (return _outhit))
    (:CastFailed
      (return ""))))

(fn ReloadFinished
  (bind _self self)
  (bind _returnvalue (Utilities|GetClass _self))
  (bind _currentammo (Utilities|GetClassDefaults _returnvalue))
  (Variables|Reload|SetReloading false)
  (if (> (Variables|Default|GetTotalAmmo) _currentammo)
    (Development|PrintString "Hello")
    (Variables|Default|SetCurrentAmmo _currentammo)
    (else
      (Development|PrintString "Bye")
      (Variables|Default|SetCurrentAmmo (Variables|Reload|GetAmmoToReload))))
  (Variables|Default|SetTotalAmmo (- (Variables|Default|GetTotalAmmo) (Variables|Reload|GetAmmoToReload)))
  (Variables|Default|SetFireActive true))

(fn OnRepReloading
  (if (Variables|Reload|GetReloading)
    (Variables|Default|SetFireActive false)
    (if (CallFunction|AbletoReload)
      (Development|PrintString "IDiot")
      (bind _returnvalue (Utilities|Time|SetTimerbyFunctionName 0 "Reload_Finished" (Variables|Reload|GetReloadTime)))
      (Variables|Reload|SetReloadTimer _returnvalue)
      (Variables|Reload|SetAmmoToReload (Math|Integer|Min(Integer) (- (Utilities|GetClassDefaults (Utilities|GetClass self)) (Variables|Default|GetCurrentAmmo)) (Variables|Default|GetTotalAmmo)))
      (else
        (Variables|Reload|SetReloading false)
        (Development|PrintString "Not Able")))))

(fn AbletoReload
  (return (and (!= (Utilities|GetClassDefaults (Utilities|GetClass self)) (Variables|Default|GetCurrentAmmo)) (> (Variables|Default|GetTotalAmmo) 0))))

(fn SpawnShootProjectile
  (bind _asmy_character (Utilities|Casting|CastToMy_Character (Game|GetInstigator)))
  (Game|SpawnActorfromClass (Variables|Default|GetFireProjectile) (Math|Transform|MakeTransform (+ (Transformation|GetWorldLocation (Variables|/Game/Blueprints/Character/My_Character.My_Character_C|GetFirstPersonCamera _asmy_character)) (* (Transformation|GetActorForwardVector (Components|GetOwner)) (Math|Conversions|ToVector(Float) 5e+01))) (Math|Conversions|RotationFromXVector (Transformation|GetActorForwardVector (Components|GetOwner)))) "Undefined" self (Variables|Default|GetDamage) (Game|GetInstigator)))