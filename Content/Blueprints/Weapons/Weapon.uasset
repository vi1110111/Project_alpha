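; Weapon Blueprint, apparently a base class, handling ammo use, fire-rate limiting and auto-fire, with empty aim stubs.
; UseWeapon decrements ammo and starts a StopRateDelay timer, which clears the rate lock and re-fires while AutoFire and FireActive hold.
; StopUseWeapon clears the firing flags; UsingWeapon has an empty OnRep.
; UseWeapon's condition is hardwired true, so AbleToUseWeapon's ammo and rate check is never applied.
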(event EventBeginPlay)

(event Collision|EventActorBeginOverlap
  (params (OtherActor :type Actor%20Object%20Reference)))

(event EventTick
  (params (DeltaSeconds :type Float%20%28single-precision%29)))

(fn ConstructionScript)

(fn UseWeapon
  (if true
    (Math|Integer|DecrementInt (Variables|Default|GetCurrentAmmo)
      (:%20%20
        (Variables|Default|SetUsingWeapon true)
        (Utilities|Time|SetTimerbyFunctionName 0 "StopRateDelay" (Variables|Default|GetUseRate))
        (Variables|Default|SetUseFreezedByRate true)
        (if (Variables|Default|GetAutoFire)
          (Variables|Default|SetFireActive true))
        (return true)))
    (else
      (Variables|Default|SetFireActive false)
      (return false))))

(fn AbletoUseWeapon
  (return (and (> (Variables|Default|GetCurrentAmmo) 0) (not (Variables|Default|GetUseFreezedByRate)))))

(fn StopRateDelay
  (Variables|Default|SetUseFreezedByRate false)
  (if (and (Variables|Default|GetAutoFire) (Variables|Default|GetFireActive))
    (CallFunction|UseWeapon)))

(fn StopUseWeapon
  (Variables|Default|SetFireActive false)
  (Variables|Default|SetUsingWeapon false))

(fn UseAim
  (if (CallFunction|AbletoUseAim)
    _))

(fn AbletoUseAim
  (return false))

(fn StopUseAim
  (return false))

(fn OnRepUsingWeapon)