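; My_Character is a first-person character Blueprint that handles mouse look and weapon input.
; On BeginPlay, its WeaponComponent creates and selects an auto rifle.
; Fire uses the current weapon when it is usable and not reloading, and stops it on release, while Reload sets the Reloading flag on BP_FireWeapons.
; GetVisibleMesh returns the first-person mesh.
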(event EventBeginPlay
  (bind _weapon (Default|CreateWeapon (Variables|Default|GetWeapon_Component) "/Game/Blueprints/Weapons/Weapon_AutoRifles.Weapon_AutoRifles_C"))
  (Default|SelectWeapon (Variables|Default|GetWeapon_Component) _weapon))

(event Input|ActionEvents|InputActionFire
  (params (Key :type Key%20Structure :default "None"))
  (bind _weapon_component (Variables|Default|GetWeapon_Component))
  (bind _currentweapon (Variables|/Game/Blueprints/Components/Player/Weapon_Component.Weapon_Component_C|GetCurrentWeapon _weapon_component))
  (:Pressed
    (bind _asbp_fire_weapons (Utilities|Casting|CastToBP_FireWeapons _currentweapon)
      (:then
        _)
      (:CastFailed
        _))
    (if (and (not (Variables|/Game/Blueprints/Weapons/BP_FireWeapons.BP_FireWeapons_C|GetReloading _asbp_fire_weapons)) (Default|AbletoUseWeapon _currentweapon))
      (Default|UseWeapon _currentweapon)))
  (:Released
    (Default|StopUseWeapon _currentweapon)))

(event Input|ActionEvents|InputActionReload
  (params (Key :type Key%20Structure :default "None"))
  (:Pressed
    (bind _asbp_fire_weapons (Utilities|Casting|CastToBP_FireWeapons (Variables|/Game/Blueprints/Components/Player/Weapon_Component.Weapon_Component_C|GetCurrentWeapon (Variables|Default|GetWeapon_Component))))
    (Variables|/Game/Blueprints/Weapons/BP_FireWeapons.BP_FireWeapons_C|SetReloading _asbp_fire_weapons true)))

(event Input|AxisEvents|InputAxisMouseX
  (params (AxisValue :type Float%20%28single-precision%29))
  (Pawn|Input|AddControllerYawInput AxisValue))

(event Input|AxisEvents|InputAxisMouseY
  (params (AxisValue :type Float%20%28single-precision%29))
  (Pawn|Input|AddControllerPitchInput AxisValue))

(fn ConstructionScript)

(fn GetVisibleMesh
  (return (Variables|Default|GetFirstPersonMesh)))