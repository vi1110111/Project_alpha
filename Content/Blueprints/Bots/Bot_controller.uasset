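; Controller for Bot pawns that sends its controlled Bot to the actor tagged "First_Destination".
; Every Tick it casts the controlled pawn to Bot, looks up the target and reissues AIMoveTo.
; FindTargetByName scans all actors in the level on each call and returns the first with the given tag.
; A delayed SpawnAIFromClass for Bot is present but unconnected, so it never runs.
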(event EventBeginPlay)

(event EventTick
  (params (DeltaSeconds :type Float%20%28single-precision%29))
  (bind _asbot (Utilities|Casting|CastToBot (Pawn|GetControlledPawn)))
  (Variables|Default|SetBot_1 _asbot)
  (bind _target (CallFunction|FindTargetbyName "First_Destination"))
  (AI|AIMoveTo (Variables|Default|GetBot_1) "0, 0, 0" _target 1e+01 false))

(fn ConstructionScript)

(fn FindTargetbyName
  (params (Tag :type Name))
  (bind _outactors (Actor|GetAllActorsOfClass "/Script/Engine.Actor"))
  (bind _array_element (Utilities|Array|ForEachLoopwithBreak _outactors :!label _label)
    (:LoopBody
      (if (Actor|ActorHasTag _array_element Tag)
        (LocalVariables|SetNewLocalVar_0 _array_element)
        (goto _label Break)))
    (:Completed
      (return (LocalVariables|GetNewLocalVar_0)))))