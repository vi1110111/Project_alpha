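; BP_Base is a HUD Blueprint that puts a UMG widget on the owning player's screen when play begins.
; ToggleHud lazily creates the widget from HUDwidgetClass, caches it and adds it to the viewport, or removes it from its parent when hiding.
; DrawHUD does nothing, and leftover text-drawing and health-reading nodes are unconnected.
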(event Collision|EventActorBeginOverlap
  (params (OtherActor :type Actor%20Object%20Reference)))

(event EventTick
  (params (DeltaSeconds :type Float%20%28single-precision%29)))

(event EventDrawHUD
  (params (SizeX :type Integer) (SizeY :type Integer)))

(event EventBeginPlay
  (CallFunction|ToggleHud true))

(fn ConstructionScript)

(fn ToggleHud
  (params (show :type Boolean))
  (if show
    (bind _hudwidget (Variables|Default|GetHUDwidget)
      (:then
        (UserInterface|Viewport|AddtoViewport _hudwidget 0))
      (:else
        (bind _returnvalue (UserInterface|CreateWidget (Variables|Default|GetHUDwidgetClass) (Game|Player|GetOwningPlayerController)))
        (bind _output_get (Variables|Default|SetHUDwidget _returnvalue))
        (UserInterface|Viewport|AddtoViewport _output_get 0)))
    (else
      (Widget|RemovefromParent (Variables|Default|GetHUDwidget)))))